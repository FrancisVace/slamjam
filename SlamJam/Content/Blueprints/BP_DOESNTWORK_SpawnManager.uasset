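; Spawn manager, named as non-working, that places actors at randomly chosen TargetPoints when play begins.
; It gathers every TargetPoint, then loops by ActorCount, spawning ActorsToSpawn at a random point and removing that point to avoid reuse.
; It prints a warning if no points exist.
; Unconnected nodes hold a Green/Red/Blue child-actor class select and a tag-based point lookup, so neither runs.
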(event `self.ReceiveBeginPlay`
  ;[1 1 1] https://www.youtube.com/watch?v=KhC8Ujoh1B8 - Checks for selected places to spawn, if 0 will remind. Randomly selects an actor to spawn and places it in one of the nominated locations (target points)
  (bind _outactors (`GameplayStatics.GetAllActorsOfClass` "/Script/Engine.TargetPoint"))
  (set `self.placesToSpawn` _outactors)
  (if (> (`KismetArrayLibrary.Array_Length` (`self.placesToSpawn`)) 0)
    (bind _result (`/Engine/EditorBlueprintResources/StandardMacros.DecrementInt` (`self.actorCount`))
      (:`  `
        (for _ (range (+ _result 1))
          (bind _output_get (set `self.currentSpawnPoint` (`KismetArrayLibrary.Array_Random` (`self.placesToSpawn`))))
          (`|SpawnActorFromClass` (`self.actorsToSpawn`) (`self.GetTransform` _output_get) "Undefined" "OverrideRootScale" null null)
          (`KismetArrayLibrary.Array_RemoveItem` (`self.placesToSpawn`) (`self.currentSpawnPoint`)))))
    (else
      (`KismetSystemLibrary.PrintString` "Forgot to set places to spawn!"))))

(fn `UserConstructionScript`)