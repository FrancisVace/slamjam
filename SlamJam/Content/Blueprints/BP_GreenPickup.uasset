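; Green speed pickup that temporarily boosts the walk speed of a BP_PlayerWorker overlapping its Collision component.
; The BoostDuration timeline drives the character's MaxWalkSpeed.
; Meanwhile, the GreenPickup component turns invisible and non-colliding, and the actor is destroyed after a delay so the timeline can keep running.
; A DoOnce limits the 2D blip sound to the first overlap, since overlaps may recur while hidden.
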(event `self.Collision.OnComponentBeginOverlap`
  (params (OverlappedComponent :type "PrimitiveComponent Object Reference") (OtherActor :type "Actor Object Reference") (OtherComp :type "PrimitiveComponent Object Reference") (OtherBodyIndex :type Integer) (bFromSweep :type Boolean) (SweepResult :type "HitResult Structure (by ref)"))
  (bind _greenpickup (`self.GreenPickup`))
  (bind _asbp_third_person_character (cast `/Game/ThirdPerson/Blueprints/BP_PlayerWorker` OtherActor))
  (`|ExecutionSequence`
    (:`then_0`
      ;[0.1366 1 0] Timeline sets the max walk speed of player character to 1200 for 5 seconds
      (bind (_direction _newtrack_0) (`Timeline|Boost Duration`)
        (:`Update`
          (set `CharacterMovementComponent.MaxWalkSpeed` _newtrack_0 (`Character.CharacterMovement` _asbp_third_person_character)))))
    (:`then_1`
      ;[0.05992 1 0] Temporarily sets the pick up to invisible and no longer supports collision for the duration, deletes when done (wouldn't work destroying without timer due to timeline functionality
      (`SceneComponent.SetVisibility` _greenpickup false false)
      (`PrimitiveComponent.SetCollisionEnabled` _greenpickup "NoCollision")
      (`KismetSystemLibrary.Delay` 5.25)
      (`self.K2_DestroyActor`))
    (:`then_2`
      ;[0.09154 1 0] Only play sound on first overlap so it doesn't do it while it's hidden
      (`/Engine/EditorBlueprintResources/StandardMacros.DoOnce` false
        (:`Completed`
          (`GameplayStatics.PlaySound2D` "/Game/Audio/SFX/DakotaSauvé-SAGAJ20-SFX-Blip_Mid.DakotaSauvé-SAGAJ20-SFX-Blip_Mid" 1.0 1.0 0.0 null null))))))

(fn `UserConstructionScript`)